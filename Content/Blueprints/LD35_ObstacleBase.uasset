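; Base obstacle actor that damages the player pawn on collision and can be captured until it has been nudged.
; BeginPlay applies the configured mesh and binds its hit event; only the first player hit deals ObstacleCollide point damage and triggers ReceiveNudge.
; ReceiveNudge disables capture, releases the mesh's physics constraint mode and sends it tumbling with random linear and angular impulses.
; Captured destroys the actor while capture is still allowed.
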(event Custom|Captured
  (params (Pawn :type Pawn%20Object%20Reference))
  (if (Variables|Default|GetCanCapture)
    (Actor|DestroyActor)))

(event Custom|ReceiveNudge
  (bind _returnvalue (Math|Random|RandomUnitVector))
  (bind _obstaclemesh (Variables|Default|GetObstacleMesh))
  (Variables|Default|SetCanCapture false)
  (Class|PrimitiveComponent|SetConstraintMode _obstaclemesh "None")
  (Physics|AddImpulse _obstaclemesh (* _returnvalue 3e+02) "None" true)
  (Class|PrimitiveComponent|AddAngularImpulse _obstaclemesh (* _returnvalue 1e+01) "None" true))

(event Custom|OnComponentHit_Event_0
  (params (OtherActor :type Actor%20Object%20Reference) (OtherComp :type Primitive%20Component%20Object%20Reference) (NormalImpulse :type Vector) (Hit :type Hit%20Result%20Structure%20%28by%20ref%29))
  (bind _asld35_player_pawn (Utilities|Casting|CastToLD35_PlayerPawn OtherActor))
  (Utilities|FlowControl|DoOnce false
    (:Completed
      (CallFunction|ReceiveNudge)
      (Game|Damage|ApplyPointDamage _asld35_player_pawn 1.0 NormalImpulse Hit 0 0 "/Game/Blueprints/ObstacleCollide.ObstacleCollide_C"))))

(event EventBeginPlay
  (Components|StaticMesh|SetStaticMesh (Variables|Default|GetObstacleMesh) (Variables|Default|GetObstacleType))
  (Collision|AssignOnComponentHit (Variables|Default|GetObstacleMesh) (delegate Custom|OnComponentHit_Event_0)))

(fn ConstructionScript)