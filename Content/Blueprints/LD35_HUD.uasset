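; LD35_HUD is a HUD that shows a red health readout for every player in the match.
; On DrawHUD it loops over the LD35_GameState player array and reads Health from each LD35_PlayerState.
; Each readout is stacked by array index near the left edge, with a red line drawn to it from the default start point.
; A few leftover math nodes are unused.
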(event EventDrawHUD
  (params (SizeX :type Integer) (SizeY :type Integer))
  (bind _returnvalue (* SizeX 0.05))
  (bind _linearcolor (Utilities|Struct|MakeLinearColor 1.0 0.0 0.0 1.0))
  (bind _asld35_game_state (Utilities|Casting|CastToLD35_GameState (Game|GetGameState)))
  (for (_array_element _array_index) (Variables|/Script/Engine.GameState|GetPlayerArray _asld35_game_state)
    (bind _asld35_player_state (Utilities|Casting|CastToLD35_PlayerState _array_element))
    (HUD|DrawText (Utilities|String|ToString(Text) (Utilities|Text|FormatText "Health {0}" (Utilities|Text|ToText(Integer) (Variables|/Game/Blueprints/LD35_PlayerState.LD35_PlayerState_C|GetHealth _asld35_player_state)))) _linearcolor _returnvalue (* (+ _array_index 1) 2e+01) 0 1.0 false)
    (Class|HUD|DrawLine 0.0 0.0 _returnvalue (* (+ _array_index 1) 2e+01) _linearcolor)))

(fn ConstructionScript)