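; LD35_ObstacleSpawn is a spawner actor that launches LD35_ObstacleBase obstacles along its arrow at ImpulseSpeed.
; On the authority only, a self-rescheduling timer waits a random delay between spawns and keeps running while spawning is toggled off.
; Each obstacle takes the spawner's transform, optionally with random roll, and a type from GetRandomObstacleToSpawn.
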(event Custom|SpawnObstacle
  (bind _returnvalue (Transformation|GetActorTransform))
  (bind (_location _rotation _scale) (Math|Transform|BreakTransform _returnvalue))
  (if (Variables|Default|GetActive)
    (Game|SpawnActorfromClass "/Game/Blueprints/LD35_ObstacleBase.LD35_ObstacleBase_C" (select (Variables|Default|GetRandomRotation) (Math|Transform|MakeTransform _location (Math|Rotator|MakeRotator (Math|Random|RandomFloatinRange 0.0 3.6e+02) (.pitch _rotation) (.yaw _rotation)) _scale) (Math|Transform|MakeTransform _location (Math|Rotator|MakeRotator (.roll _rotation) (.pitch _rotation) (.yaw _rotation)) _scale)) "Undefined" 0 (|GetRandomObstacleToSpawn) (Math|Vector|RotateVector (Math|Vector|MakeVector (Variables|Default|GetImpulseSpeed) 0.0 0.0) (Transformation|GetWorldRotation (Variables|Default|GetArrow))))
    (CallFunction|NextSpawnDelay)))

(event Custom|NextSpawnDelay
  (Utilities|Time|SetTimerbyEvent (delegate Custom|SpawnObstacle) (Math|Random|RandomFloatinRange (Variables|Default|GetMinDelay) (Variables|Default|GetMaxDelay))))

(event Custom|ToggleSpawning
  (params (Active :type Boolean))
  (Variables|Default|SetActive Active))

(event EventBeginPlay
  (Networking|SwitchHasAuthority
    (:Authority
      (CallFunction|NextSpawnDelay))))

(fn ConstructionScript)