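; LD35_PlayerPawn is the player's pawn, a procedurally generated box that takes damage when it hits obstacles.
; BeginPlay builds the Shape mesh section from GenerateBoxMesh with collision enabled.
; Hits from LD35_ObstaclePawn apply ObstacleCollide point damage to the pawn and clear the obstacle cube's constraint mode.
; The PointDamage event subtracts the floored damage from Health on LD35_PlayerState.
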(event OnComponentHit(Shape)
  (params (OtherActor :type Actor%20Object%20Reference) (OtherComp :type Primitive%20Component%20Object%20Reference) (NormalImpulse :type Vector) (Hit :type Hit%20Result%20Structure%20%28by%20ref%29))
  (bind _asld35_obstacle_pawn (Utilities|Casting|CastToLD35_ObstaclePawn OtherActor))
  (Game|Damage|ApplyPointDamage self 1e+01 NormalImpulse Hit 0 OtherActor "/Game/Blueprints/ObstacleCollide.ObstacleCollide_C")
  (Class|PrimitiveComponent|SetConstraintMode (Variables|/Game/Blueprints/LD35_ObstaclePawn.LD35_ObstaclePawn_C|GetCube _asld35_obstacle_pawn) "None"))

(event Game|Damage|EventPointDamage
  (params (Damage :type Float%20%28single-precision%29) (DamageType :type Damage%20Type%20Object%20Reference) (HitLocation :type Vector :default "0, 0, 0") (HitNormal :type Vector :default "0, 0, 0") (HitComponent :type Primitive%20Component%20Object%20Reference) (BoneName :type Name :default "None") (ShotFromDirection :type Vector :default "0, 0, 0") (InstigatedBy :type Controller%20Object%20Reference) (DamageCauser :type Actor%20Object%20Reference))
  (bind _returnvalue (Pawn|GetController))
  (bind _playerstate (Variables|/Script/Engine.Controller|GetPlayerState _returnvalue))
  (bind _asld35_player_state (Utilities|Casting|CastToLD35_PlayerState _playerstate))
  (Variables|/Game/Blueprints/LD35_PlayerState.LD35_PlayerState_C|SetHealth _asld35_player_state (- (Variables|/Game/Blueprints/LD35_PlayerState.LD35_PlayerState_C|GetHealth _asld35_player_state) (Math|Float|Floor Damage))))

(event EventBeginPlay
  (bind (_vertices _triangles _normals _uvs _tangents) (Class|KismetProceduralMeshLibrary|GenerateBoxMesh "10.000000,5.000000,5.000000"))
  (Class|ProceduralMeshComponent|CreateMeshSection (Variables|Default|GetShape) 0 _vertices _triangles _normals _uvs 0 _tangents true))

(event EventActorBeginOverlap
  (params (OtherActor :type Actor%20Object%20Reference)))

(event EventTick
  (params (DeltaSeconds :type Float%20%28single-precision%29)))

(fn ConstructionScript)